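; Boss enemy Blueprint that adds an enemy HUD widget to the viewport on BeginPlay and fires projectiles automatically.
; Chained Delay nodes on Tick act as cooldowns, ignoring retriggers while pending.
; The FireRate delay paces paired shots from the Top and Bottom points with a shot sound.
; A further delay gates a larger, more damaging Center shot with an explosion sound.
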(event `self.ReceiveBeginPlay`
  (`parent.ReceiveBeginPlay`)
  (bind _returnvalue (`|CreateWidget` "/Game/UI/HUDEnemy.HUDEnemy_C"))
  (bind _output_get (set `self.HudReference` _returnvalue))
  (`UserWidget.AddToViewport` _output_get 0))

(event `self.ReceiveTick`
  (params (DeltaSeconds :type "Float (single-precision)"))
  (`parent.ReceiveTick` DeltaSeconds)
  (`KismetSystemLibrary.Delay` (`self.FireRate`))
  (`|SpawnActorFromClass` "/Game/Blueprints/Projectiles/bpProjectileEnemy.bpProjectileEnemy_C" (`SceneComponent.K2_GetComponentToWorld` (`self.Top`)) "AdjustIfPossibleButAlwaysSpawn" "OverrideRootScale" null 5.0 (0.0 -2000.0 0.0) (1.0 1.0 1.0) null)
  (`|SpawnActorFromClass` "/Game/Blueprints/Projectiles/bpProjectileEnemy.bpProjectileEnemy_C" (`SceneComponent.K2_GetComponentToWorld` (`self.Bottom`)) "AdjustIfPossibleButAlwaysSpawn" "OverrideRootScale" null 5.0 (0.0 -2000.0 0.0) (1.0 1.0 1.0) null)
  (`GameplayStatics.PlaySoundAtLocation` "/Game/Audio/EnemyShot.EnemyShot")
  (`KismetSystemLibrary.Delay` 3.0)
  (`|SpawnActorFromClass` "/Game/Blueprints/Projectiles/bpProjectileEnemy.bpProjectileEnemy_C" (`SceneComponent.K2_GetComponentToWorld` (`self.Center`)) "AdjustIfPossibleButAlwaysSpawn" "OverrideRootScale" null 10.0 (0.0 -2000.0 0.0) (3.0 3.0 3.0) null)
  (`GameplayStatics.PlaySoundAtLocation` "/Game/Audio/Explosion.Explosion"))

(fn `UserConstructionScript`
  (`parent.UserConstructionScript`))