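; A pickup actor that drifts at a default speed along the Y axis until it detects the player, then homes in on them.
; Overlapping its box with a bpPlayer stores that player reference once.
; Each tick, it blends the ProjectileMovement velocity halfway toward the player's direction scaled by IncreaseSpeed.
; No collection or reward logic is implemented here.
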(event `self.ReceiveTick`
  (params (DeltaSeconds :type "Float (single-precision)"))
  (bind _projectilemovement (`self.ProjectileMovement`))
  (`/Engine/EditorBlueprintResources/StandardMacros.IsValid` (`self.bpPlayerReference`)
    (:`Is Valid`
      (set `MovementComponent.Velocity` (`KismetMathLibrary.VLerp` (`MovementComponent.Velocity` (`self.ProjectileMovement`)) (* (`KismetMathLibrary.Normal` (- (`self.K2_GetActorLocation` (`self.bpPlayerReference`)) (`self.K2_GetActorLocation`))) (`self.IncreaseSpeed`)) 0.5) _projectilemovement))
    (:`Is Not Valid`
      (set `MovementComponent.Velocity` (`KismetMathLibrary.MakeVector` 0.0 (`self.DefaultSpeed`)) _projectilemovement))))

(event `self.Box.OnComponentBeginOverlap`
  (params (OverlappedComponent :type "PrimitiveComponent Object Reference") (OtherActor :type "Actor Object Reference") (OtherComp :type "PrimitiveComponent Object Reference") (OtherBodyIndex :type Integer) (bFromSweep :type Boolean) (SweepResult :type "HitResult Structure (by ref)"))
  (bind _asbp_player (cast `/Game/Blueprints/Misc/bpPlayer` OtherActor))
  (`/Engine/EditorBlueprintResources/StandardMacros.IsValid` (`self.bpPlayerReference`)
    (:`Is Not Valid`
      (set `self.bpPlayerReference` _asbp_player))))

(fn `UserConstructionScript`)