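; Game mode Blueprint that handles camera shake requests and the response to all enemies being defeated.
; CallCamShake plays the given shake as a world camera shake.
; AllEnemiesDefeated opens Level1 when the current level is Main, otherwise it creates the passed-in widget.
; The nodes that would display that widget, show the cursor and set UI input are disconnected, so they never run.
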(event `CallCamShake`
  (params (ShakeType :type "CameraShake Class Reference"))
  (`GameplayStatics.PlayWorldCameraShake` ShakeType (0.0 0.0 0.0) -1.0 500.0))

(event `AllEnemiesDefeated`
  (params (WidgetToShow :type "UserWidget Class Reference"))
  (bind _returnvalue (`GameplayStatics.GetCurrentLevelName` true))
  (if (not (`KismetStringLibrary.EqualEqual_StrStr` _returnvalue "Main"))
    (bind _returnvalue_2 (`|CreateWidget` WidgetToShow))
    (else
      (`GameplayStatics.OpenLevel` "Level1"))))

(fn `UserConstructionScript`)