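; Game mode that tracks score and coins, plays background music and spawns an island at a random height on BeginPlay.
; Coins load from a save slot at start and save at EndPlay, though the re-save after loading passes the coin count as UserIndex.
; When all enemies are defeated, it opens Level1 from Main; elsewhere it creates a widget, but the viewport and input-mode steps are unwired.
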(event `self.ReceiveBeginPlay`
  (`self.LoadCoins`)
  (`AudioComponent.Play` (`self.BGM`) 0.0)
  (`self.SpawnIsland`))

(event `self.ReceiveEndPlay`
  (params (EndPlayReason :type "EEndPlayReason Enum" :default "Destroyed"))
  (`self.SaveCoins`))

(event `CallCamShake`
  (params (ShakeType :type "CameraShake Class Reference"))
  (`GameplayStatics.PlayWorldCameraShake` ShakeType (0.0 0.0 0.0) -1.0 500.0))

(event `AllEnemiesDefeated`
  (params (WidgetToShow :type "UserWidget Class Reference"))
  (bind _returnvalue (`GameplayStatics.GetCurrentLevelName` true))
  (if (not (`KismetStringLibrary.EqualEqual_StrStr` _returnvalue "Main"))
    (bind _returnvalue_2 (`|CreateWidget` WidgetToShow))
    (else
      (`GameplayStatics.OpenLevel` "Level1"))))

(fn `AddCoin`
  (set `self.Coins` (+ (`self.Coins`) 1)))

(fn `AddScore`
  (set `self.Score` (+ (`self.Score`) 10)))

(fn `LoadCoins`
  (bind _returnvalue (`GameplayStatics.DoesSaveGameExist` (`self.CoinSaveName`)))
  (if _returnvalue
    (bind _returnvalue_2 (`GameplayStatics.LoadGameFromSlot` (`self.CoinSaveName`)))
    (bind _output_get (set `self.SaveGameSub` _returnvalue_2))
    (bind _asbp_coin_save (cast `/Game/Blueprints/Misc/bpCoinSave` _output_get))
    (bind _output_get_2 (set `self.Coins` (`/Game/Blueprints/Misc/bpCoinSave.CoinsCount` _asbp_coin_save)))
    (`GameplayStatics.SaveGameToSlot` (`self.SaveGameSub`) (`self.CoinSaveName`) _output_get_2)
    (else
      (`self.SaveCoins`))))

(fn `ResetScoresAndCoins`
  (set `self.Score` 0)
  (set `self.Coins` 0))

(fn `SaveCoins`
  (bind _returnvalue (`GameplayStatics.CreateSaveGameObject` "/Game/Blueprints/Misc/bpCoinSave.bpCoinSave_C"))
  (bind _output_get (set `self.SaveGameSub` _returnvalue))
  (bind _asbp_coin_save (cast `/Game/Blueprints/Misc/bpCoinSave` _output_get))
  (set `/Game/Blueprints/Misc/bpCoinSave.CoinsCount` (`self.Coins`) _asbp_coin_save)
  (`GameplayStatics.SaveGameToSlot` (`self.SaveGameSub`) (`self.CoinSaveName`)))

(fn `SpawnIsland`
  (`|SpawnActorFromClass` "/Game/Blueprints/Misc/bpIsland.bpIsland_C" (`KismetMathLibrary.MakeTransform` (`KismetMathLibrary.MakeVector` 21000.0 35000.0 (`KismetMathLibrary.RandomFloatInRange` -2500.0 2500.0))) "Undefined" "OverrideRootScale" null null))

(fn `UserConstructionScript`)