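; Enemy spawner actor that runs up to five sequential waves, each with its own enemy count and class pool.
; A looping timer polls the game mode and starts the next wave once no live enemies remain and the spawner is ready.
; BeginWave publishes the wave total to the game mode, then SpawnWave spawns random classes in one loop at fixed X/Y and random Z, re-arming the spawner when done.
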(event `self.ReceiveBeginPlay`
  ;[0.5285 1 0.3379] Event BeginPlay -: Spawn Wave
  (bind _asbp_game_mode (cast `/Game/Blueprints/Misc/bpGameMode` (`GameplayStatics.GetGameMode`)))
  (set `self.bpGameMode` _asbp_game_mode)
  (bind _returnvalue (`KismetSystemLibrary.K2_SetTimer` null "WaveCheck" 0.5 true))
  (set `self.WaveTimer` _returnvalue))

(event `WaveCheck`
  (bind _output (`|GetArrayItem` (`self.WaveEnemyCount`) (`self.WaveIndex`)))
  ;[1 1 1] Wave Check
  (if (and (== (`/Game/Blueprints/Misc/bpGameMode.LiveEnemies` (`self.bpGameMode`)) 0) (`self.bWaveReady`))
    (switch `int` (`self.WaveIndex`)
      (:`0`
        (`self.BeginWave` _output)
        (`self.SpawnWave` _output (`self.WaveEnemies1`)))
      (:`1`
        (`self.BeginWave` _output)
        (`self.SpawnWave` _output (`self.WaveEnemies2`)))
      (:`2`
        (`self.BeginWave` _output)
        (`self.SpawnWave` _output (`self.WaveEnemies3`)))
      (:`3`
        (`self.BeginWave` _output)
        (`self.SpawnWave` _output (`self.WaveEnemies4`)))
      (:`4`
        (`self.BeginWave` _output)
        (`self.SpawnWave` _output (`self.WaveEnemies5`))))
    (set `self.WaveIndex` (+ (`self.WaveIndex`) 1))))

(fn `BeginWave`
  (params (WaveTotal :type Integer))
  (bind _bpgamemode (`self.bpGameMode`))
  ;[1 1 1] BeginWave
  (set `self.bWaveReady` false)
  (set `self.WaveActive` 0)
  (set `/Game/Blueprints/Misc/bpGameMode.MaxWaves` WaveTotal _bpgamemode)
  (set `/Game/Blueprints/Misc/bpGameMode.ActiveWave` WaveTotal _bpgamemode))

(fn `SpawnWave`
  (params (WaveTotal :type Integer) (WaveEnemies :type "Array of /Game/Blueprints/Enemy/bpEnemyBase Class Reference"))
  (bind _bpgamemode (`self.bpGameMode`))
  (bind (_enemyspawnlocationmin_x _enemyspawnlocationmin_y _enemyspawnlocationmin_z) (`KismetMathLibrary.BreakVector` (`/Game/Blueprints/Misc/bpGameMode.EnemySpawnLocationMin` _bpgamemode)))
  (bind (_enemyspawnlocationmax_x _enemyspawnlocationmax_y _enemyspawnlocationmax_z) (`KismetMathLibrary.BreakVector` (`/Game/Blueprints/Misc/bpGameMode.EnemySpawnLocationMax` _bpgamemode)))
  ;[1 1 1] SpawnWave
  (for _ (range (+ (+ WaveTotal 1) 1))
    (if (> WaveTotal (`self.WaveActive`))
      (if (not (`self.bWaveReady`))
        (`|SpawnActorFromClass` (`|GetArrayItem` WaveEnemies (`KismetMathLibrary.RandomInteger` (`KismetArrayLibrary.Array_Length` WaveEnemies))) (`KismetMathLibrary.MakeTransform` (`KismetMathLibrary.MakeVector` _enemyspawnlocationmin_x _enemyspawnlocationmin_y (`KismetMathLibrary.RandomFloatInRange` _enemyspawnlocationmin_z _enemyspawnlocationmax_z))) "Undefined" "OverrideRootScale" null null)
        (set `self.WaveActive` (+ (`self.WaveActive`) 1)))
      (else
        (set `self.bWaveReady` true)))))

(fn `UserConstructionScript`)